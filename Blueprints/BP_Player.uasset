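; BP_Player is the player pawn Blueprint, handling walking and looking input.
; Walking axes feed movement input along the Camera component's forward and right vectors, so the forward direction includes any camera pitch.
; Looking axes drive controller rotation with names crossed: Looking_UpDown adds yaw and Looking_RightLeft adds pitch.
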(event `InputAxis|Walking_ForwardBackward`
  (params (AxisValue :type "Float (single-precision)"))
  (`self.AddMovementInput` (`SceneComponent.GetForwardVector` (`self.Camera`)) AxisValue))

(event `InputAxis|Walking_RightLeft`
  (params (AxisValue :type "Float (single-precision)"))
  (`self.AddMovementInput` (`SceneComponent.GetRightVector` (`self.Camera`)) AxisValue))

(event `InputAxis|Looking_UpDown`
  (params (AxisValue :type "Float (single-precision)"))
  (`self.AddControllerYawInput` AxisValue))

(event `InputAxis|Looking_RightLeft`
  (params (AxisValue :type "Float (single-precision)"))
  (`self.AddControllerPitchInput` AxisValue))

(fn `UserConstructionScript`)